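; Pirate character Blueprint that moves itself along one axis once the Enter key starts it walking.
; Pressing Enter sets a small movement speed and flags the character as walking.
; Tick feeds that speed into movement input along the right vector of the control yaw until IsFinished is true, a flag this graph never sets.
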(event EventBeginPlay)

(event Collision|EventActorBeginOverlap
  (params (OtherActor :type Actor%20Object%20Reference)))

(event EventTick
  (params (DeltaSeconds :type Float%20%28single-precision%29))
  ;[1 1 1] Start Walking
  (if (not (Variables|Default|GetIs_Finished))
    (Pawn|Input|AddMovementInput (Math|Vector|GetRightVector (Math|Rotator|MakeRotator 0.0 0.0 (.Yaw (Math|Rotator|BreakRotator (Pawn|GetControlRotation :!class /Script/Engine.Pawn))))) (Variables|Default|GetMovementSpeed) false)))

(event Input|KeyboardEvents|Enter
  (params (Key :type Key%20Structure))
  ;[1 1 1] Start Walking
  (:Pressed
    (Variables|Default|SetMovementSpeed 0.1)
    (Variables|Default|SetIs_Walking true)))

(fn ConstructionScript)